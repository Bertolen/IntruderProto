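; FBP_Ladder is a ladder actor that assembles its visual mesh procedurally from a configurable segment count.
; The construction script stacks segments vertically by MeshHeight, adding instances to separate bottom, straight, attach and top instanced mesh components.
; The first and last segments become the bottom and top caps, with an attach piece at every index divisible by three between them.
; The event graph holds no active logic.
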(fn `UserConstructionScript`
  (bind _returnvalue (- (`self.AmountLadderMesh`) 1))
  (for _index (range (+ _returnvalue 1))
    (if (== _index 0)
      (bind _returnvalue_2 (`KismetMathLibrary.MakeTransform` (`KismetMathLibrary.MakeVector` 0.0 0.0 (* _index (`self.MeshHeight`)))))
      (`InstancedStaticMeshComponent.AddInstance` (`self.LadderBottom`) _returnvalue_2)
      (elif (== _index _returnvalue)
        (`InstancedStaticMeshComponent.AddInstance` (`self.LadderTop`) _returnvalue_2)
        (elif (== (mod _index 3) 0)
          (`InstancedStaticMeshComponent.AddInstance` (`self.LadderAttach`) _returnvalue_2)
          (else
            (`InstancedStaticMeshComponent.AddInstance` (`self.LadderStraight`) _returnvalue_2)))))))